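; Tutorial decal actor that fades magic text through a timeline when something overlaps its trigger.
; On BeginPlay it draws DecalText into a CRT_MagicText canvas render target and feeds that texture to a dynamic decal material.
; TextTrigger overlap plays TL_Magicfade to drive Fade, once or repeatedly per CanRepeat, never while already playing.
; The BP_Player cast is disconnected, so any actor triggers it, with a debug print.
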(event `self.ReceiveBeginPlay`
  (bind _returnvalue (`CanvasRenderTarget2D.CreateCanvasRenderTarget2D` "/Game/Blueprint/Tutorial_Text/RenderTargets/CRT_MagicText.CRT_MagicText_C" 1024 512))
  (bind _ascrt_magic_text (cast `/Game/Blueprint/Tutorial_Text/RenderTargets/CRT_MagicText` _returnvalue))
  (bind _output_get (set `self.CR_DecalText` _ascrt_magic_text))
  (set `/Game/Blueprint/Tutorial_Text/RenderTargets/CRT_MagicText.TextTodraw` (`self.DecalText`) _output_get)
  (`CanvasRenderTarget2D.UpdateResource` _output_get)
  (bind _returnvalue_2 (`DecalComponent.CreateDynamicMaterialInstance` (`self.MagicDecal`)))
  (bind _output_get_2 (set `self.DecalMaterial` _returnvalue_2))
  ;[0.8125 0.3032 0.05501 0.5 25] Scalar Parameter vom Material bestimmen
  (`MaterialInstanceDynamic.SetTextureParameterValue` _output_get_2 "TextTexture" _output_get)
  (`MaterialInstanceDynamic.SetScalarParameterValue` _output_get_2 "Fade" 0.0)
  (`MaterialInstanceDynamic.SetScalarParameterValue` _output_get_2 "UseImage" 0.0))

(event `self.TextTrigger.OnComponentBeginOverlap`
  (params (OverlappedComponent :type "PrimitiveComponent Object Reference") (OtherActor :type "Actor Object Reference") (OtherComp :type "PrimitiveComponent Object Reference") (OtherBodyIndex :type Integer) (bFromSweep :type Boolean) (SweepResult :type "HitResult Structure (by ref)"))
  (`KismetSystemLibrary.PrintString` "aaahh")
  (if (and (not (`self.IsPlaying`)) (or (not (`self.HasTriggered`)) (`self.CanRepeat`)))
    (set `self.HasTriggered` true)
    (set `self.IsPlaying` true)
    (bind (_direction _fadevalue) (`Timeline|TL_Magicfade` :!via `PlayFromStart`)
      (:`Update`
        (`MaterialInstanceDynamic.SetScalarParameterValue` (`self.DecalMaterial`) "Fade" _fadevalue))
      (:`Finished`
        (set `self.IsPlaying` false)))))

(fn `UserConstructionScript`)