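; Interactable soul companion that talks to the player and can start or stop following them through dialogue actions.
; Interact drives an indexed dialogue list with choices in a typewriter widget, then runs the last entry's action when dialogue ends.
; Overlap with FollowCollider and that follow state toggle Tick, which steps toward the player outside StopRadius with clamped height and smoothed facing.
; A timeline bobs the mesh root as idle animation.
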(event OnComponentBeginOverlap(FollowCollider)
  (params (OverlappedComponent :type Primitive%20Component%20Object%20Reference) (OtherActor :type Actor%20Object%20Reference) (OtherComp :type Primitive%20Component%20Object%20Reference) (OtherBodyIndex :type Integer) (bFromSweep :type Boolean) (SweepResult :type Hit%20Result%20Structure%20%28by%20ref%29))
  ;[0.15 0.15 0.15 0.5] BeginOverlap
  (Utilities|Casting|CastToBP_Player OtherActor)
  (Variables|Movement|GetDidInteractWithSoul
    (:then
      (Variables|Movement|SetCanFollowPlayer true)
      (Actor|Tick|SetActorTickEnabled true))
    (:else)))

(event OnComponentEndOverlap(FollowCollider)
  (params (OverlappedComponent :type Primitive%20Component%20Object%20Reference) (OtherActor :type Actor%20Object%20Reference) (OtherComp :type Primitive%20Component%20Object%20Reference) (OtherBodyIndex :type Integer))
  ;[0.15 0.15 0.15 0.5] EndOverlap
  (Utilities|Casting|CastToBP_Player OtherActor)
  (Variables|Movement|SetCanFollowPlayer false)
  (Actor|Tick|SetActorTickEnabled false))

(event Custom|IdleSoul
  ;[0.15 0.15 0.15 0.5] IdleAnimation
  (bind _move (Timeline|MoveUpDownT Play)
    (:Update
      (Transformation|SetRelativeLocation (Variables|Default|GetMeshroot) (Math|Vector|MakeVector 0.0 0.0 (* _move (Variables|Movement|GetIdleHight))) false false))))

(event Custom|StartDialogue
  (bind _returnvalue (Viewport|GetViewportSize))
  (bind (_x _y) (Math|Vector2D|BreakVector2D _returnvalue))
  ;[0.15 0.15 0.15 0.5] Start Dialogue
  (Math|Integer|IncrementInt (Variables|/Game/Character/BP/BP_Player.BP_Player_C|GetCanMove (Variables|Default|GetPlayerRef))
    (:%20%20
      (Variables|Movement|SetIsTalking true)
      (Variables|Dialogue|SetTalkList 0)
      (Variables|Dialogue|GetCAWDialogueRef
        (:then
          _)
        (:else
          (Class|PlayerController|SetMouseLocation (Game|GetPlayerController 0) (Math|Float|Truncate (/ _x 2.0)) (Math|Float|Truncate (/ _y 2.0)))
          (bind _returnvalue_2 (Class|CommonActivatableWidgetContainerBase|AddWidget (Utilities|ReturnMainStack (Game|GetPlayerController 0)) "/Game/Blueprint/UI/Dialogue/CAW_Dialogue.CAW_Dialogue_C"))
          (bind _output_get (Variables|Dialogue|SetCAWDialogueRef _returnvalue_2))
          (EventDispatchers|BindEventtoOnDialogueChoiceSelected _output_get (EventDispatchers|CreateEvent :!event HandleDialogueChoice))))
      (Input|SetInputModeGameandUI (Game|GetPlayerController 0) 0 "DoNotLock" false false)
      (Variables|/Script/Engine.PlayerController|SetbShowMouseCursor (Game|GetPlayerController 0) true)
      (CallFunction|SetDialogueText))))

(event Custom|NextDialogue
  (bind _dialogueentries (Variables|Dialogue|GetDialogueEntries))
  (bind _cawdialogueref (Variables|Dialogue|GetCAWDialogueRef))
  ;[0.15 0.15 0.15 0.5] NextDialogue
  (Variables|/Game/Blueprint/UI/Dialogue/CAW_Dialogue.CAW_Dialogue_C|GetIsTyping _cawdialogueref
    (:then
      (Default|FinishTypewriter _cawdialogueref))
    (:else
      (Utilities|FlowControl|Delay 0.1)
      (if (Utilities|Array|IsValidIndex _dialogueentries (Variables|Dialogue|GetTalkList))
        (if (== (Utilities|Array|Length (.Coices (Utilities|Struct|BreakST_DialogueEntry (Utilities|Array|Get(acopy) _dialogueentries (Variables|Dialogue|GetTalkList))))) 0)
          (if (Utilities|Array|IsValidIndex (Variables|Dialogue|GetDialogueEntries) (.NextDialogueIndex (Utilities|Struct|BreakST_DialogueEntry (Utilities|Array|Get(acopy) _dialogueentries (Variables|Dialogue|GetTalkList)))))
            (Variables|Dialogue|SetTalkList (.NextDialogueIndex (Utilities|Struct|BreakST_DialogueEntry (Utilities|Array|Get(acopy) _dialogueentries (Variables|Dialogue|GetTalkList)))))
            (CallFunction|SetDialogueText)
            (else
              (CallFunction|EndDialogue :!label _label))))
        (else
          (goto _label))))))

(event Custom|EndDialogue
  (bind _returnvalue (Game|GetPlayerController 0))
  ;[0.15 0.15 0.15 0.5] EndDialogue
  (bind _cawdialogueref (Variables|Dialogue|GetCAWDialogueRef)
    (:then
      (Class|CommonActivatableWidgetContainerBase|RemoveWidget (Utilities|ReturnMainStack (Game|GetPlayerController 0)) _cawdialogueref)
      (Input|SetInputModeGameOnly _returnvalue true)
      (Variables|/Script/Engine.PlayerController|SetbShowMouseCursor _returnvalue false)
      (Variables|Dialogue|SetCAWDialogueRef 0)
      (Variables|Movement|SetIsTalking false)
      (Math|Integer|DecrementInt (Variables|/Game/Character/BP/BP_Player.BP_Player_C|GetCanMove (Variables|Default|GetPlayerRef))
        (:%20%20
          (if (Utilities|Array|IsValidIndex (Variables|Dialogue|GetDialogueEntries) (Variables|Dialogue|GetTalkList))
            (CallFunction|ExecuteDialogueAction (.DialogueAction (Utilities|Struct|BreakST_DialogueEntry (Utilities|Array|Get(acopy) (Variables|Dialogue|GetDialogueEntries) (Variables|Dialogue|GetTalkList))))))
          (Variables|Dialogue|SetTalkList 0))))
    (:else)))

(event EventBeginPlay
  ;[0.05286 0.2384 0.05448] BeginPlay
  (bind _asbp_player (Utilities|Casting|CastToBP_Player (Game|GetPlayerCharacter 0)))
  (Variables|Default|SetPlayerRef _asbp_player)
  ;[0.15 0.15 0.15 0.5] UpDownPlayrate
  (CallFunction|IdleSoul)
  (Components|Timeline|SetPlayRate (Variables|Default|GetMoveUpDownT) (|(1/{C026E1DC-426C-3CF2-2F4C-17B97979D733}))))

(event EventInteract
  (params (Send :type Actor%20Object%20Reference))
  ;[0.15 0.15 0.15 0.5] OnInteract
  (bind _asbp_player (Utilities|Casting|CastToBP_Player Send))
  (Variables|Default|SetPlayerRef _asbp_player)
  (Variables|Movement|GetIsTalking
    (:then
      (CallFunction|NextDialogue))
    (:else
      (CallFunction|StartDialogue))))

(event EventTick
  (params (DeltaSeconds :type Float%20%28single-precision%29))
  (bind _self self)
  (bind _soulspeed (Variables|Movement|GetSoulSpeed))
  (bind _playerref (Variables|Default|GetPlayerRef))
  (bind _returnvalue (Transformation|GetActorLocation _playerref))
  (bind _returnvalue_2 (Transformation|GetActorLocation _self))
  (bind _returnvalue_3 (- _returnvalue _returnvalue_2))
  (bind _returnvalue_4 (Math|Vector|Normalize _returnvalue_3))
  (bind _returnvalue_5 (* _returnvalue_4 _soulspeed))
  (bind _returnvalue_6 (+ _returnvalue_5 _returnvalue_2))
  ;[0.05364 0.2396 0.05416] Event Tick
  (Variables|Movement|SetDeltaSeconds DeltaSeconds)
  (if (> (Math|Vector|Distance(Vector) (Transformation|GetActorLocation self) (Transformation|GetActorLocation (Variables|Default|GetPlayerRef))) (Variables|Movement|GetStopRadius))
    (Transformation|SetActorLocation (Math|Vector|MakeVector (.x _returnvalue_6) (.y _returnvalue_6) (Math|Float|Clamp(Float) (.z _returnvalue_6) 8e+01 1.2e+02)) false false)
    (Transformation|SetActorRotation (Math|Interpolation|RInterpTo (Transformation|GetActorRotation) (Math|Rotator|FindLookatRotation (Transformation|GetActorLocation) (Transformation|GetActorLocation (Variables|Default|GetPlayerRef))) (Variables|Movement|GetDeltaSeconds) 3.0))))

(fn ConstructionScript)

(fn SetDialogueText
  (bind _dialogueentries (Variables|Dialogue|GetDialogueEntries))
  (bind _talklist (Variables|Dialogue|GetTalkList))
  (bind _output (Utilities|Array|Get(acopy) _dialogueentries _talklist))
  (bind (_dialoguetext _nextdialogueindex _coices) (Utilities|Struct|BreakST_DialogueEntry _output))
  (if (Utilities|Array|IsValidIndex (Variables|Dialogue|GetDialogueEntries) (Variables|Dialogue|GetTalkList))
    (Default|StartTypewriter (Variables|Dialogue|GetCAWDialogueRef) _dialoguetext _coices)))

(fn HandleDialogueChoice
  (params (NextDialogueIndex :type Integer))
  (if (Utilities|Array|IsValidIndex (Variables|Dialogue|GetDialogueEntries) NextDialogueIndex)
    (Variables|Dialogue|SetTalkList NextDialogueIndex)
    (CallFunction|SetDialogueText)
    (else
      (CallFunction|EndDialogue))))

(fn ExecuteDialogueAction
  (params (Action :type E_DialogueAction%20Enum :default "NewEnumerator0"))
  (switch Utilities|FlowControl|Switch|SwitchonE_DialogueAction Action
    (:NewEnumerator1
      (Variables|Movement|SetDidInteractWithSoul true)
      (if (Collision|IsOverlappingActor (Variables|Default|GetFollowCollider) (Variables|Default|GetPlayerRef) :!class /Script/Engine.PrimitiveComponent)
        (Variables|Movement|SetCanFollowPlayer true)
        (Actor|Tick|SetActorTickEnabled true)))
    (:NewEnumerator2
      (Variables|Movement|SetDidInteractWithSoul false)
      (Variables|Movement|SetCanFollowPlayer false)
      (Actor|Tick|SetActorTickEnabled false))))

(fn ReturnInteractStatus
  (return (Variables|Movement|GetCan%20Interact)))