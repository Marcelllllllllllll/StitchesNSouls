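; BP_DeadZone is a world damage zone that repeatedly damages the player while they overlap its DamageZone component.
; On begin overlap it stores the player, adds itself uniquely to the player's ActiveDamageZones array and starts a looping timer, if none is active, to apply damage at a set interval.
; On end overlap it clears the timer through StopDamageTimer and removes itself from that array.
; ReturnInteractStatus always returns false.
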(event `DealZoneDamage`
  (bind _playerref (`self.PlayerRef`)
    (:`then`
      (`GameplayStatics.ApplyDamage` _playerref (`self.DamageAmount`)))
    (:`else`)))

(event `self.DamageZone.OnComponentBeginOverlap`
  (params (OverlappedComponent :type "PrimitiveComponent Object Reference") (OtherActor :type "Actor Object Reference") (OtherComp :type "PrimitiveComponent Object Reference") (OtherBodyIndex :type Integer) (bFromSweep :type Boolean) (SweepResult :type "HitResult Structure (by ref)"))
  (bind _asbp_player (cast `/Game/Character/BP/BP_Player` OtherActor))
  (set `self.PlayerRef` _asbp_player)
  (`KismetArrayLibrary.Array_AddUnique` (`/Game/Character/BP/BP_Player.ActiveDamageZones` _asbp_player) self) ; Verhindert das dieselbe Damage Zone Referenz mehrfach im Array landet
  (if (not (`KismetSystemLibrary.K2_IsTimerActiveHandle` (`self.DamageTimerHandle`)))
    (bind _returnvalue (`KismetSystemLibrary.K2_SetTimerDelegate` (`|CreateDelegate` :!event `DealZoneDamage`) (`self.DamageInterval`) true))
    (set `self.DamageTimerHandle` _returnvalue)))

(event `self.DamageZone.OnComponentEndOverlap`
  (params (OverlappedComponent :type "PrimitiveComponent Object Reference") (OtherActor :type "Actor Object Reference") (OtherComp :type "PrimitiveComponent Object Reference") (OtherBodyIndex :type Integer))
  (bind _asbp_player (cast `/Game/Character/BP/BP_Player` OtherActor))
  (`self.StopDamageTimer`)
  (`KismetArrayLibrary.Array_RemoveItem` (`/Game/Character/BP/BP_Player.ActiveDamageZones` _asbp_player) self))

(fn `ReturnInteractStatus`
  (returns (CanInteract :type Boolean))
  (return false))

(fn `StopDamageTimer`
  (`KismetSystemLibrary.K2_ClearAndInvalidateTimerHandle` (`self.DamageTimerHandle`)))

(fn `UserConstructionScript`)